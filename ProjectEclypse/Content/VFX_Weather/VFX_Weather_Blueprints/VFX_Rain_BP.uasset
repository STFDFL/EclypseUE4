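; Rain effect actor that exposes a single SpawnRate value to control its rain particle system.
; The construction script pushes SpawnRate to the particle component, with a second emitter parameter, SpawnRate2, set to five times that value.
; Tick compares SpawnRate against a cached LastSpawnRate and reapplies both parameters only when it changes, so rain intensity can vary at runtime.
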(event EventBeginPlay)

(event EventActorBeginOverlap
  (params (OtherActor :type Actor%20Object%20Reference)))

(event EventTick
  (params (DeltaSeconds :type Float%20%28single-precision%29))
  (if (not (== (Variables|Default|GetLastSpawnRate) (Variables|Default|GetSpawnRate)))
    (Variables|Default|SetLastSpawnRate (Variables|Default|GetSpawnRate))
    (Effects|Components|ParticleSystem|SetFloatParameter (Variables|Default|GetBP_Rain_PS) "SpawnRate" (Variables|Default|GetSpawnRate))
    (Effects|Components|ParticleSystem|SetFloatParameter (Variables|Default|GetBP_Rain_PS) "SpawnRate2" (* (Variables|Default|GetSpawnRate) 5.0))))

(fn ConstructionScript
  (bind _bp_rain_ps (Variables|Default|GetBP_Rain_PS))
  (bind _spawnrate (Variables|Default|GetSpawnRate))
  (Effects|Components|ParticleSystem|SetFloatParameter _bp_rain_ps "SpawnRate" _spawnrate)
  (Effects|Components|ParticleSystem|SetFloatParameter _bp_rain_ps "SpawnRate2" (* _spawnrate 5.0)))