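; Camera actor Blueprint with unfinished or disconnected mouse-look logic, so it has no active behavior as wired.
; The Look Up/Down and Left/Right axis events are empty, as are BeginPlay and the construction script.
; Orphaned nodes would enable input, show the cursor, toggle SetCameraMovable and add axis values to pitch and yaw while that flag is set, but none of them run.
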(event EventBeginPlay)

(event Collision|EventActorBeginOverlap
  (params (OtherActor :type Actor%20Object%20Reference)))

(event EventTick
  (params (DeltaSeconds :type Float%20%28single-precision%29)))

(event Input|AxisEvents|InputAxisLookLeft/Right
  (params (AxisValue :type Float%20%28single-precision%29))
  ;[1 1 1] Added MouseLook
)

(event Input|AxisEvents|InputAxisLookUp/Down
  (params (AxisValue :type Float%20%28single-precision%29))
  ;[1 1 1] Added MouseLook
)

(event Input|MouseEvents|RightMouseButton
  (params (Key :type Key%20Structure :default "AnyKey")))

(fn ConstructionScript)