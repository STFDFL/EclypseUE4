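; BP_Wall_Light_001 is a tavern wall light with a point light, a spot light and a candle flame particle.
; The construction script shows or hides all three from the Lit flag and sets the spot light's shadow casting from a CastShadows setting.
; On BeginPlay, a timeline drives the point light's intensity.
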(event EventBeginPlay
  (bind _light_intensity (Timeline|Timeline_0 Play)
    (:Update
      (Rendering|Components|Light|SetIntensity (Variables|Default|GetPointLight) _light_intensity))))

(event EventActorBeginOverlap
  (params (OtherActor :type Actor%20Object%20Reference)))

(event EventTick
  (params (DeltaSeconds :type Float%20%28single-precision%29)))

(fn ConstructionScript
  (if (Variables|Default|GetLit)
    (Rendering|SetVisibility (Variables|Default|GetPointLight) true false)
    (else
      (Rendering|SetVisibility (Variables|Default|GetP_Candle_Flame_001) false false)))
  (Rendering|Components|Light|SetCastShadows (Variables|Default|GetSpotLight) (Variables|Default|GetCast%20Shadows)))