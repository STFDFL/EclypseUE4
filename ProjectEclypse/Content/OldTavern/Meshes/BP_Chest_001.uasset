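; BP_Chest_001 is a configurable tavern chest prop whose state is set entirely in the construction script.
; A LockChest flag shows or hides the Lock component.
; An OpenChest0Closed1Open value, clamped to 0–1, blends the Chest2 component's roll from closed to 110 degrees open.
; The event graph is empty, so the chest has no runtime opening logic.
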(event EventBeginPlay)

(event EventActorBeginOverlap
  (params (OtherActor :type Actor%20Object%20Reference)))

(event EventTick
  (params (DeltaSeconds :type Float%20%28single-precision%29)))

(fn ConstructionScript
  (bind _lock (Variables|Default|Getlock))
  (if (Variables|Default|GetLock%20Chest)
    (Rendering|SetVisibility _lock true false)
    (else
      (Rendering|SetVisibility _lock false false)))
  (Transformation|SetRelativeRotation (Variables|Default|GetChest2) (Math|Rotator|Lerp(Rotator) (Math|Rotator|MakeRotator 0.0 0.0 0.0) (Math|Rotator|MakeRotator -1.1e+02 0.0 0.0) (Math|Float|Clamp(Float) (Variables|Default|GetOpen%20Chest%200=Closed%201=Open))) false false))