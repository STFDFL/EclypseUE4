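; Modular roof piece for the Old Village structures, configured entirely in the construction script.
; ChooseComponent selects left, middle, right, top, end or bend variants, setting the mesh, offset and roof, interior or exterior material overrides per slot.
; Straight pieces share an X/Y scale adjustment; bends skip it and add hand-placed pole meshes.
; Middle End sets only the roof material, and Left/Right mostly use opposite-lettered R/L meshes.
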(event EventBeginPlay)

(event EventActorBeginOverlap
  (params (OtherActor :type Actor%20Object%20Reference)))

(event EventTick
  (params (DeltaSeconds :type Float%20%28single-precision%29)))

(fn ConstructionScript
  (bind _staticmesh (Variables|Default|GetStaticMesh))
  (bind _staticmesh_2 (Variables|Default|GetStaticMesh))
  (bind _staticmesh3 (Variables|Default|GetStaticMesh3))
  (bind _staticmesh4 (Variables|Default|GetStaticMesh4))
  (bind _staticmesh_3 (Variables|Default|GetStaticMesh))
  (bind _staticmesh_4 (Variables|Default|GetStaticMesh))
  (bind _staticmesh1 (Variables|Default|GetStaticMesh1))
  (bind _staticmesh_5 (Variables|Default|GetStaticMesh))
  (bind _staticmesh_6 (Variables|Default|GetStaticMesh))
  (bind _staticmesh_7 (Variables|Default|GetStaticMesh))
  (bind _staticmesh_8 (Variables|Default|GetStaticMesh))
  (bind _staticmesh_9 (Variables|Default|GetStaticMesh))
  (bind _staticmesh_10 (Variables|Default|GetStaticMesh))
  (bind _staticmesh_11 (Variables|Default|GetStaticMesh))
  (bind _staticmesh_12 (Variables|Default|GetStaticMesh))
  (bind _staticmesh_13 (Variables|Default|GetStaticMesh))
  (bind _staticmesh_14 (Variables|Default|GetStaticMesh))
  (bind _staticmesh1_2 (Variables|Default|GetStaticMesh1))
  (bind _staticmesh_15 (Variables|Default|GetStaticMesh))
  (bind _staticmesh_16 (Variables|Default|GetStaticMesh))
  (bind _staticmesh_17 (Variables|Default|GetStaticMesh))
  (bind _staticmesh_18 (Variables|Default|GetStaticMesh))
  (bind _staticmesh_19 (Variables|Default|GetStaticMesh))
  (bind _staticmesh_20 (Variables|Default|GetStaticMesh))
  (bind _staticmesh_21 (Variables|Default|GetStaticMesh))
  (bind _staticmesh_22 (Variables|Default|GetStaticMesh))
  (bind _staticmesh_23 (Variables|Default|GetStaticMesh))
  (bind _staticmesh1_3 (Variables|Default|GetStaticMesh1))
  (bind _staticmesh2 (Variables|Default|GetStaticMesh2))
  (switch Utilities|FlowControl|Switch|SwitchonBP_Roof_Enum (Variables|Default|GetChoose%20Component)
    (:NewEnumerator3
      ;[1 1 1] Left 01
      (Components|StaticMesh|SetStaticMesh _staticmesh_5 "/Game/OldVillage/Meshes/Structure_Components/SM_Roof_R_001.SM_Roof_R_001")
      (Transformation|SetRelativeTransform _staticmesh_5 (Math|Transform|MakeTransform "100.000000,0.000000,0.000000" "0,-90.000000, 0" "1,1.000000,1") false false)
      (Rendering|Material|SetMaterial _staticmesh_3 1 (Variables|Default|GetExterior%20Material%20Override))
      (Rendering|Material|SetMaterial _staticmesh_3 0 (Variables|Default|GetInterior%20Material%20Override))
      (Rendering|Material|SetMaterial (Variables|Default|GetStaticMesh) 4 (Variables|Default|GetRoof%20Material%20Override))
      ;[1 1 1] Set lenght and Scale
      (Transformation|SetWorldScale3D (Variables|Default|GetStaticMesh) (Math|Vector|MakeVector (+ 0.0 (Variables|Default|GetScale%20adjust%20X)) (+ 0.0 (Variables|Default|GetScale%20adjust%20Y)) 1.0) :!label _label))
    (:NewEnumerator6
      ;[1 1 1] Left 02
      (Components|StaticMesh|SetStaticMesh _staticmesh_22 "/Game/OldVillage/Meshes/Structure_Components/SM_Roof_R_002.SM_Roof_R_002")
      (Transformation|SetRelativeTransform _staticmesh_22 (Math|Transform|MakeTransform "-20.000000,0.000000,0.000000" "0,-90.000000, 0" "1,1.000000,1") false false)
      (Rendering|Material|SetMaterial (Variables|Default|GetStaticMesh) 2 (Variables|Default|GetRoof%20Material%20Override))
      (goto _label))
    (:NewEnumerator0
      ;[1 1 1] Left End
      (Components|StaticMesh|SetStaticMesh _staticmesh_15 "/Game/OldVillage/Meshes/Structure_Components/SM_Roof_End_R_001.SM_Roof_End_R_001")
      (Transformation|SetRelativeTransform _staticmesh_15 (Math|Transform|MakeTransform "100.000000,0.000000,0.000000" "0,-90.000000, 0" "1,1.000000,1") false false)
      (Rendering|Material|SetMaterial (Variables|Default|GetStaticMesh) 3 (Variables|Default|GetRoof%20Material%20Override))
      (Rendering|Material|SetMaterial _staticmesh_8 0 (Variables|Default|GetInterior%20Material%20Override))
      (Rendering|Material|SetMaterial _staticmesh_8 1 (Variables|Default|GetExterior%20Material%20Override))
      (goto _label))
    (:NewEnumerator13
      ;[1 1 1] Left 01 top
      (Components|StaticMesh|SetStaticMesh _staticmesh_6 "/Game/OldVillage/Meshes/Structure_Components/SM_Roof_L_Top_001.SM_Roof_L_Top_001")
      (Transformation|SetRelativeTransform _staticmesh_6 (Math|Transform|MakeTransform "0.000000,0.000000,0.000000" "0,0.000000, 0" "1,1.000000,1") false false)
      (Rendering|Material|SetMaterial (Variables|Default|GetStaticMesh) 0 (Variables|Default|GetRoof%20Material%20Override))
      (Rendering|Material|SetMaterial _staticmesh_9 4 (Variables|Default|GetInterior%20Material%20Override))
      (Rendering|Material|SetMaterial _staticmesh_9 3 (Variables|Default|GetExterior%20Material%20Override))
      (goto _label))
    (:NewEnumerator10
      ;[1 1 1] Left 02 Cap
      (Components|StaticMesh|SetStaticMesh _staticmesh_23 "/Game/OldVillage/Meshes/Structure_Components/SM_Roof_L_002_Cap.SM_Roof_L_002_Cap")
      (Transformation|SetRelativeTransform _staticmesh_23 (Math|Transform|MakeTransform "-20.000000,0.000000,0.000000" "0,-90.000000, 0" "1,1.000000,1") false false)
      (Rendering|Material|SetMaterial (Variables|Default|GetStaticMesh) 2 (Variables|Default|GetRoof%20Material%20Override))
      (goto _label))
    (:NewEnumerator4
      ;[1 1 1] Middle 01
      (Components|StaticMesh|SetStaticMesh _staticmesh_16 "/Game/OldVillage/Meshes/Structure_Components/SM_Roof_M_001.SM_Roof_M_001")
      (Transformation|SetRelativeTransform _staticmesh_16 (Math|Transform|MakeTransform "100.000000,0.000000,0.000000" "0,-90.000000, 0" "1,1.000000,1") false false)
      (Rendering|Material|SetMaterial (Variables|Default|GetStaticMesh) 0 (Variables|Default|GetRoof%20Material%20Override))
      (goto _label))
    (:NewEnumerator7
      ;[1 1 1] Middle 02
      (Components|StaticMesh|SetStaticMesh _staticmesh_19 "/Game/OldVillage/Meshes/Structure_Components/SM_Roof_M_002.SM_Roof_M_002")
      (Transformation|SetRelativeTransform _staticmesh_19 (Math|Transform|MakeTransform "100.000000,0.000000,0.000000" "0,-90.000000, 0" "1,1.000000,1") false false)
      (Rendering|Material|SetMaterial (Variables|Default|GetStaticMesh) 0 (Variables|Default|GetRoof%20Material%20Override))
      (goto _label))
    (:NewEnumerator15
      ;[1 1 1] Middle 01 top
      (Components|StaticMesh|SetStaticMesh _staticmesh_7 "/Game/OldVillage/Meshes/Structure_Components/SM_Roof_M_Top_001.SM_Roof_M_Top_001")
      (Transformation|SetRelativeTransform _staticmesh_7 (Math|Transform|MakeTransform "0.000000,0.000000,0.000000" "0,0.000000, 0" "1,1.000000,1") false false)
      (Rendering|Material|SetMaterial (Variables|Default|GetStaticMesh) 0 (Variables|Default|GetRoof%20Material%20Override))
      (Rendering|Material|SetMaterial _staticmesh_13 2 (Variables|Default|GetInterior%20Material%20Override))
      (Rendering|Material|SetMaterial _staticmesh_13 3 (Variables|Default|GetExterior%20Material%20Override))
      (goto _label))
    (:NewEnumerator1
      (Rendering|Material|SetMaterial (Variables|Default|GetStaticMesh) 1 (Variables|Default|GetRoof%20Material%20Override)))
    (:NewEnumerator5
      ;[1 1 1] Right 01
      (Components|StaticMesh|SetStaticMesh _staticmesh "/Game/OldVillage/Meshes/Structure_Components/SM_Roof_L_001.SM_Roof_L_001")
      (Transformation|SetRelativeTransform _staticmesh (Math|Transform|MakeTransform "120.000000,0.000000,0.000000" "0,-90.000000, 0" "1,1.000000,1") false false)
      (Rendering|Material|SetMaterial (Variables|Default|GetStaticMesh) 4 (Variables|Default|GetRoof%20Material%20Override))
      (Rendering|Material|SetMaterial _staticmesh_11 0 (Variables|Default|GetInterior%20Material%20Override))
      (Rendering|Material|SetMaterial _staticmesh_11 1 (Variables|Default|GetExterior%20Material%20Override))
      (goto _label))
    (:NewEnumerator8
      ;[1 1 1] Right 02 1m
      (Components|StaticMesh|SetStaticMesh _staticmesh_21 "/Game/OldVillage/Meshes/Structure_Components/SM_Roof_L_002.SM_Roof_L_002")
      (Transformation|SetRelativeTransform _staticmesh_21 (Math|Transform|MakeTransform "120.000000,0.000000,0.000000" "0,-90.000000, 0" "1,1.000000,1") false false)
      (Rendering|Material|SetMaterial (Variables|Default|GetStaticMesh) 2 (Variables|Default|GetRoof%20Material%20Override))
      (goto _label))
    (:NewEnumerator2
      ;[1 1 1] Right End
      (Components|StaticMesh|SetStaticMesh _staticmesh_17 "/Game/OldVillage/Meshes/Structure_Components/SM_Roof_End_L_001.SM_Roof_End_L_001")
      (Transformation|SetRelativeTransform _staticmesh_17 (Math|Transform|MakeTransform "100.000000,0.000000,0.000000" "0,-90.000000, 0" "1,1.000000,1") false false)
      (Rendering|Material|SetMaterial (Variables|Default|GetStaticMesh) 3 (Variables|Default|GetRoof%20Material%20Override))
      (Rendering|Material|SetMaterial _staticmesh_12 0 (Variables|Default|GetInterior%20Material%20Override))
      (Rendering|Material|SetMaterial _staticmesh_12 1 (Variables|Default|GetExterior%20Material%20Override))
      (goto _label))
    (:NewEnumerator14
      ;[1 1 1] Right 01 top
      (Components|StaticMesh|SetStaticMesh _staticmesh_18 "/Game/OldVillage/Meshes/Structure_Components/SM_Roof_R_Top_001.SM_Roof_R_Top_001")
      (Transformation|SetRelativeTransform _staticmesh_18 (Math|Transform|MakeTransform "0.000000,0.000000,0.000000" "0,0.000000, 0" "1,1.000000,1") false false)
      (Rendering|Material|SetMaterial (Variables|Default|GetStaticMesh) 0 (Variables|Default|GetRoof%20Material%20Override))
      (Rendering|Material|SetMaterial _staticmesh_10 4 (Variables|Default|GetInterior%20Material%20Override))
      (Rendering|Material|SetMaterial _staticmesh_10 3 (Variables|Default|GetExterior%20Material%20Override))
      (goto _label))
    (:NewEnumerator9
      ;[1 1 1] Right 02 cap
      (Components|StaticMesh|SetStaticMesh _staticmesh_20 "/Game/OldVillage/Meshes/Structure_Components/SM_Roof_R_002_Cap.SM_Roof_R_002_Cap")
      (Transformation|SetRelativeTransform _staticmesh_20 (Math|Transform|MakeTransform "120.000000,0.000000,0.000000" "0,-90.000000, 0" "1,1.000000,1") false false)
      (Rendering|Material|SetMaterial (Variables|Default|GetStaticMesh) 2 (Variables|Default|GetRoof%20Material%20Override))
      (goto _label))
    (:NewEnumerator11
      ;[1 1 1] 45 bend
      (Components|StaticMesh|SetStaticMesh _staticmesh_4 "/Game/OldVillage/Meshes/Structure_Components/SM_Roof_Turn_45_001.SM_Roof_Turn_45_001")
      (Transformation|SetRelativeTransform _staticmesh_4 (Math|Transform|MakeTransform "0.000000,0.000000,0.000000" "0,-90.000000, 0" "1,1.000000,1") false false)
      (Components|StaticMesh|SetStaticMesh _staticmesh1 "/Game/OldVillage/Meshes/Structure_Components/SM_Pole_003.SM_Pole_003")
      (Transformation|SetRelativeTransform _staticmesh1 (Math|Transform|MakeTransform "0.871933,-225.344147,107.858498" "-4.958731,-2.902614,115.594124" "1.929088,2.317508,3.112247") false false)
      (Components|StaticMesh|SetStaticMesh _staticmesh2 "/Game/OldVillage/Meshes/Structure_Components/SM_Pole_003.SM_Pole_003")
      (Transformation|SetRelativeTransform _staticmesh2 (Math|Transform|MakeTransform "22.016939,-224.254028,113.026634" "-63.206715,-108.537262,170.187729" "2.139159,1.308582,3.112247") false false)
      (Components|StaticMesh|SetStaticMesh _staticmesh3 "/Game/OldVillage/Meshes/Structure_Components/SM_Pole_003.SM_Pole_003")
      (Transformation|SetRelativeTransform _staticmesh3 (Math|Transform|MakeTransform "327.038391,-147.521317,-24.954344" "-64.096443,-162.510391,8.261389" "2.139159,1.308582,3.144759") false false)
      (Components|StaticMesh|SetStaticMesh _staticmesh4 "/Game/OldVillage/Meshes/Structure_Components/SM_Pole_003.SM_Pole_003")
      (Transformation|SetRelativeTransform _staticmesh4 (Math|Transform|MakeTransform "82.687073,-311.990601,121.850372" "65.107285,6.160970,-174.832764" "2.203449,1.586636,3.112256") false false)
      (Rendering|Material|SetMaterial (Variables|Default|GetStaticMesh) 2 (Variables|Default|GetRoof%20Material%20Override)))
    (:NewEnumerator12
      ;[1 1 1] 90 bend IN
      (Components|StaticMesh|SetStaticMesh _staticmesh_14 "/Game/OldVillage/Meshes/Structure_Components/SM_Roof_Turn_90_001.SM_Roof_Turn_90_001")
      (Transformation|SetRelativeTransform _staticmesh_14 (Math|Transform|MakeTransform "0.000000,0.000000,0.000000" "0,-90.000000, 0" "1,1.000000,1") false false)
      (Components|StaticMesh|SetStaticMesh _staticmesh1_2 "/Game/OldVillage/Meshes/Structure_Components/SM_Pole_002_simple.SM_Pole_002_simple")
      (Transformation|SetRelativeTransform _staticmesh1_2 (Math|Transform|MakeTransform "271.797913,56.527878,-6.761283" "71.527092,42.000797,-2.709234" "2.382818,1.313035,4.072622") false false)
      (Rendering|Material|SetMaterial (Variables|Default|GetStaticMesh) 1 (Variables|Default|GetRoof%20Material%20Override)))
    (:NewEnumerator16
      ;[1 1 1] 90 bend OUT
      (Components|StaticMesh|SetStaticMesh _staticmesh_2 "/Game/OldVillage/Meshes/Structure_Components/SM_Roof_Turn_90_002.SM_Roof_Turn_90_002")
      (Transformation|SetRelativeTransform _staticmesh_2 (Math|Transform|MakeTransform "100.000000,0.000000,0.000000" "0,-90.000000, 0" "1,1.000000,1") false false)
      (Components|StaticMesh|SetStaticMesh _staticmesh1_3 "/Game/OldVillage/Meshes/Structure_Components/SM_Pole_001.SM_Pole_001")
      (Transformation|SetRelativeTransform _staticmesh1_3 (Math|Transform|MakeTransform "36.000000,66.925522,-24.123796" "-68.523544,-72.615730,25.867401" "0.558876,0.405526,4.100000") false false)
      (Rendering|Material|SetMaterial (Variables|Default|GetStaticMesh) 1 (Variables|Default|GetRoof%20Material%20Override)))))