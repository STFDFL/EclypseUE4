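; BP_Stairs is a configurable building piece for the OldVillage environment that places either stairs or a middle step, with abandoned mesh variants.
; Its construction script picks the mesh from ChooseComponent and AbbandonedBuilding, then scales it by Height, LenghtY and LenghtX.
; Abandoned stairs get a tinted dynamic stucco material, but the final BaseMaterialOverride assignment to the same slot replaces it.
; The event graph has no active logic.
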(event EventBeginPlay)

(event EventActorBeginOverlap
  (params (OtherActor :type Actor%20Object%20Reference)))

(event EventTick
  (params (DeltaSeconds :type Float%20%28single-precision%29)))

(fn ConstructionScript
  (switch Utilities|FlowControl|Switch|SwitchonPB_Stairs_Enum (Variables|Default|GetChoose%20component)
    (:NewEnumerator0
      (if (Variables|Default|GetAbbandoned%20Building)
        (Components|StaticMesh|SetStaticMesh (Variables|Default|Getstairs) "/Game/OldVillage/Meshes/Structure_Components/SM_Stairs_001_Abbandoned.SM_Stairs_001_Abbandoned")
        (bind _returnvalue (Rendering|Material|CreateDynamicMaterialInstance (Variables|Default|Getstairs) 0 "/Game/OldVillage/Materials/Tileable/MI_Stucco_fine_001.MI_Stucco_fine_001" :!class /Script/Engine.PrimitiveComponent))
        (Rendering|Material|SetVectorParameterValue _returnvalue "Color multyplier" "(R=0.730000,G=0.689000,B=0.565000,A=1.000000)" :!class /Script/Engine.MaterialInstanceDynamic)))
    (:NewEnumerator1
      (Components|StaticMesh|SetStaticMesh (Variables|Default|Getstairs) "/Game/OldVillage/Meshes/Structure_Components/SM_Stairs_Step_001.SM_Stairs_Step_001")
      (if (Variables|Default|GetAbbandoned%20Building)
        (Components|StaticMesh|SetStaticMesh (Variables|Default|Getstairs) "/Game/OldVillage/Meshes/Structure_Components/SM_Stairs_Step_001_abbandoned.SM_Stairs_Step_001_abbandoned"))))
  (Transformation|SetWorldScale3D (Variables|Default|Getstairs) (Math|Vector|MakeVector (Variables|Default|GetHeight) (Variables|Default|GetLenght%20Y) (Variables|Default|GetLenght%20X)))
  (Rendering|Material|SetMaterial (Variables|Default|Getstairs) 0 (Variables|Default|GetBase%20Material%20Override)))