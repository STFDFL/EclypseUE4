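; Modular 1m x 1m building wall piece that configures itself in the construction script as a basic wall, window, corner or bend.
; ChooseComponent selects the base mesh and places add-on meshes: glass, an adjustable shutter and flowers, or bars with stone or pole surrounds.
; AbbandonedBuilding swaps in derelict meshes or materials per variant.
; Interior and exterior material overrides apply first, with stucco color set through a dynamic material instance.
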(event EventBeginPlay)

(event EventActorBeginOverlap
  (params (OtherActor :type Actor%20Object%20Reference)))

(event EventTick
  (params (DeltaSeconds :type Float%20%28single-precision%29)))

(fn ConstructionScript
  (bind _static_mesh (Variables|Default|GetStatic%20Mesh))
  (bind _static_mesh_2 (Variables|Default|GetStatic%20Mesh))
  (bind _static_mesh_3 (Variables|Default|GetStatic%20Mesh))
  (bind _staticmesh2 (Variables|Default|GetStaticMesh2))
  (bind _staticmesh3 (Variables|Default|GetStaticMesh3))
  (bind _staticmesh4 (Variables|Default|GetStaticMesh4))
  (bind _exterior_material_override (Variables|Default|GetExterior%20Material%20Override))
  (bind _staticmesh5 (Variables|Default|GetStaticMesh5))
  (bind _staticmesh2_2 (Variables|Default|GetStaticMesh2))
  (bind _staticmesh3_2 (Variables|Default|GetStaticMesh3))
  (bind _staticmesh4_2 (Variables|Default|GetStaticMesh4))
  (bind _static_mesh_4 (Variables|Default|GetStatic%20Mesh))
  (bind _staticmesh5_2 (Variables|Default|GetStaticMesh5))
  (bind _staticmesh1 (Variables|Default|GetStaticMesh1))
  (bind _staticmesh2_3 (Variables|Default|GetStaticMesh2))
  (bind _staticmesh1_2 (Variables|Default|GetStaticMesh1))
  (bind _staticmesh4_3 (Variables|Default|GetStaticMesh4))
  (bind _staticmesh6 (Variables|Default|GetStaticMesh6))
  (bind _static_mesh_5 (Variables|Default|GetStatic%20Mesh))
  (bind _static_mesh_6 (Variables|Default|GetStatic%20Mesh))
  (bind _staticmesh1_3 (Variables|Default|GetStaticMesh1))
  (bind _staticmesh2_4 (Variables|Default|GetStaticMesh2))
  (bind _staticmesh3_3 (Variables|Default|GetStaticMesh3))
  (bind _staticmesh4_4 (Variables|Default|GetStaticMesh4))
  (bind _staticmesh5_3 (Variables|Default|GetStaticMesh5))
  (bind _staticmesh1_4 (Variables|Default|GetStaticMesh1))
  (bind _staticmesh2_5 (Variables|Default|GetStaticMesh2))
  (bind _staticmesh3_4 (Variables|Default|GetStaticMesh3))
  (bind _staticmesh4_5 (Variables|Default|GetStaticMesh4))
  (bind _staticmesh5_4 (Variables|Default|GetStaticMesh5))
  (bind _staticmesh2_6 (Variables|Default|GetStaticMesh2))
  (bind _staticmesh3_5 (Variables|Default|GetStaticMesh3))
  (bind _staticmesh4_6 (Variables|Default|GetStaticMesh4))
  (bind _staticmesh5_5 (Variables|Default|GetStaticMesh5))
  (bind _staticmesh7 (Variables|Default|GetStaticMesh7))
  (bind _static_mesh_7 (Variables|Default|GetStatic%20Mesh))
  (bind _staticmesh2_7 (Variables|Default|GetStaticMesh2))
  (bind _staticmesh1_5 (Variables|Default|GetStaticMesh1))
  (bind _staticmesh4_7 (Variables|Default|GetStaticMesh4))
  (bind _staticmesh6_2 (Variables|Default|GetStaticMesh6))
  (bind _static_mesh_8 (Variables|Default|GetStatic%20Mesh))
  (bind _static_mesh_9 (Variables|Default|GetStatic%20Mesh))
  (Rendering|Material|SetMaterial (Variables|Default|GetStatic%20Mesh) 0 (Variables|Default|GetInterior%20Material%20Override))
  (Rendering|Material|SetMaterial (Variables|Default|GetStatic%20Mesh) 1 _exterior_material_override)
  (bind _returnvalue (Rendering|Material|CreateDynamicMaterialInstance (Variables|Default|GetStatic%20Mesh) 1 _exterior_material_override :!class /Script/Engine.PrimitiveComponent))
  (Rendering|Material|SetVectorParameterValue _returnvalue "Material 2 Color multiplier" (Variables|Default|GetStucco%20Color%20) :!class /Script/Engine.MaterialInstanceDynamic)
  (switch Utilities|FlowControl|Switch|SwitchonBP_1mx1m_enum (Variables|Default|GetChoose%20component)
    (:NewEnumerator0
      ;[1 1 1] Basic Wall
      (if (Variables|Default|GetAbbandoned%20Building)
        (Rendering|Material|SetMaterial (Variables|Default|GetStatic%20Mesh) 0 "/Game/OldVillage/Materials/Tileable/MI_Blend_Stones_Exterior_001_to_Stucco_fine_001_parallax.MI_Blend_Stones_Exterior_001_to_Stucco_fine_001_parallax")))
    (:NewEnumerator5
      (if (Variables|Default|GetAbbandoned%20Building)
        ;[1 1 1] Window 01_Abbandoned
        ;;[1 1 1] Base
        (Components|StaticMesh|SetStaticMesh _static_mesh_4 "/Game/OldVillage/Meshes/Structure_Components/SM_wall_1mx1m_Window_001_abbandoned.SM_wall_1mx1m_Window_001_abbandoned")
        (Transformation|SetRelativeTransform _static_mesh_4 (Math|Transform|MakeTransform "0.000000,0.000000,0.000000" "0,0.000000, 0") false false)
        ;;[1 1 1] Window body
        (Components|StaticMesh|SetStaticMesh _staticmesh1 "/Game/OldVillage/Meshes/Structure_Components/SM_Window_003_abbandoned_frame.SM_Window_003_abbandoned_frame")
        (Transformation|SetRelativeTransform _staticmesh1 (Math|Transform|MakeTransform "124.371246,-16.489357,52.227348" "0.000000,-89.999992,0.000000" "0.745748,0.966496,0.956341") false false)
        (switch int (Variables|Default|GetChoose%20abbandoned%20window%20glass)
          (:1
            ;;[1 1 1] Glass
            (Components|StaticMesh|SetStaticMesh _staticmesh2_7 "/Game/OldVillage/Meshes/Structure_Components/SM_Window_003_abbandoned_glass_001.SM_Window_003_abbandoned_glass_001")
            (Transformation|SetRelativeTransform _staticmesh2_7 (Math|Transform|MakeTransform "124.371246,-16.489357,52.227348" "0.000000,-89.999992,0.000000" "0.745748,0.966496,0.956341") false false))
          (:2
            ;;[1 1 1] Glass
            (Components|StaticMesh|SetStaticMesh _staticmesh2_3 "/Game/OldVillage/Meshes/Structure_Components/SM_Window_003_abbandoned_glass_002.SM_Window_003_abbandoned_glass_002")
            (Transformation|SetRelativeTransform _staticmesh2_3 (Math|Transform|MakeTransform "124.371246,-16.489357,52.227348" "0.000000,-89.999992,0.000000" "0.745748,0.966496,0.956341") false false))
          (:3
            _))
        ;;[1 1 1] Shutters support
        (Components|StaticMesh|SetStaticMesh _staticmesh4_7 "/Game/OldVillage/Meshes/Structure_Components/SM_Window_Shutter_003_support_abbandoned.SM_Window_Shutter_003_support_abbandoned")
        (Transformation|SetRelativeTransform _staticmesh4_7 (Math|Transform|MakeTransform "66.938431,7.452263,53.735527" "0.000000,-90.000000,0.000000" "1.000000,1.000000,1.000000") false false)
        ;;[1 1 1] Remove left shutter
        (if (Variables|Default|GetRemove%20shutter)
          _
          (else
            ;;[1 1 1] Shutter
            (Components|StaticMesh|SetStaticMesh _staticmesh6_2 "/Game/OldVillage/Meshes/Structure_Components/SM_Window_Shutter_003_abbandoned.SM_Window_Shutter_003_abbandoned")
            (Transformation|SetRelativeTransform _staticmesh6_2 (Math|Transform|MakeTransform "66.938431,7.452263,53.735527" "0.000000,-90.000000,0.000000" "1.000000,1.000000,1.000000") false false)))
        (Transformation|AddLocalOffset _staticmesh6_2 "0.000000,-52.000000,-45.000000" false false)
        ;;[1 1 1] Shutters movement
        (Transformation|SetRelativeRotation _staticmesh6_2 (Math|Rotator|Lerp(Rotator) (Math|Rotator|MakeRotator 0.0 0.0 -94.0) (Math|Rotator|MakeRotator 0.0 0.0 97.0) (Math|Float|Clamp(Float) (Variables|Default|GetShutter%20-%201%20=%20Open%200%20=%20Closed))) false false)
        (else
          ;[1 1 1] Window 01
          ;;[1 1 1] Base
          (Components|StaticMesh|SetStaticMesh _static_mesh_5 "/Game/OldVillage/Meshes/Structure_Components/SM_wall_1mx1m_Window_001.SM_wall_1mx1m_Window_001")
          (Transformation|SetRelativeTransform _static_mesh_5 (Math|Transform|MakeTransform "0.000000,0.000000,0.000000" "0,0.000000, 0") false false)
          ;;[1 1 1] Window body
          (Components|StaticMesh|SetStaticMesh _staticmesh1_2 "/Game/OldVillage/Meshes/Structure_Components/SM_Window_003.SM_Window_003")
          (Transformation|SetRelativeTransform _staticmesh1_2 (Math|Transform|MakeTransform "124.371246,-16.489357,52.227348" "0.000000,-89.999992,0.000000" "0.745748,0.966496,0.956341") false false)
          ;;[1 1 1] Shutters support
          (Components|StaticMesh|SetStaticMesh _staticmesh4_3 "/Game/OldVillage/Meshes/Structure_Components/SM_Window_Shutter_003_support.SM_Window_Shutter_003_support")
          (Transformation|SetRelativeTransform _staticmesh4_3 (Math|Transform|MakeTransform "66.938431,7.452263,53.735527" "0.000000,-90.000000,0.000000" "1.000000,1.000000,1.000000") false false)
          ;;[1 1 1] Remove left shutter
          (if (Variables|Default|GetRemove%20shutter)
            _
            (else
              ;;[1 1 1] Ledt Shutter
              (Components|StaticMesh|SetStaticMesh _staticmesh6 "/Game/OldVillage/Meshes/Structure_Components/SM_Window_Shutter_003.SM_Window_Shutter_003")
              (Transformation|SetRelativeTransform _staticmesh6 (Math|Transform|MakeTransform "66.938431,7.452263,53.735527" "0.000000,-90.000000,0.000000" "1.000000,1.000000,1.000000") false false)))
          (Transformation|AddLocalOffset _staticmesh6 "0.000000,-52.000000,-45.000000" false false)
          ;;[1 1 1] Shutters movement
          (Transformation|SetRelativeRotation _staticmesh6 (Math|Rotator|Lerp(Rotator) (Math|Rotator|MakeRotator 0.0 0.0 -94.0) (Math|Rotator|MakeRotator 0.0 0.0 97.0) (Math|Float|Clamp(Float) (Variables|Default|GetShutter%20-%201%20=%20Open%200%20=%20Closed))) false false)))
      (if (Variables|Default|GetWindow%20Flowers)
        (Components|StaticMesh|SetStaticMesh _staticmesh7 "/Game/OldVillage/Meshes/Vegetation/SM_Flower__Window_004.SM_Flower__Window_004")
        (Transformation|SetRelativeTransform _staticmesh7 (Math|Transform|MakeTransform "47.657925,0.544784,12.022932" "0.000000,0.000000,0.000000" "1.000000,1.000000,1.000000") false false)))
    (:NewEnumerator6
      (if (Variables|Default|GetAbbandoned%20Building)
        ;[1 1 1] Base
        (Components|StaticMesh|SetStaticMesh _static_mesh_6 "/Game/OldVillage/Meshes/Structure_Components/SM_wall_1mx1m_Window_002_abbandoned.SM_wall_1mx1m_Window_002_abbandoned")
        (Transformation|SetRelativeTransform _static_mesh_6 (Math|Transform|MakeTransform "0.000000,0.000000,0.000000" "0,0.000000, 0") false false)
        (else
          (Components|StaticMesh|SetStaticMesh _static_mesh_7 "/Game/OldVillage/Meshes/Structure_Components/SM_wall_1mx1m_Window_002.SM_wall_1mx1m_Window_002")
          (Transformation|SetRelativeTransform _static_mesh_7 (Math|Transform|MakeTransform "0.000000,0.000000,0.000000" "0,0.000000, 0") false false)))
      (switch int (Variables|Default|GetChoose%20Bars)
        (:1
          ;[1 1 1] Bars
          (Components|StaticMesh|SetStaticMesh _staticmesh1_4 "/Game/OldVillage/Meshes/Structure_Components/SM_Bars_003.SM_Bars_003")
          (Transformation|SetRelativeTransform _staticmesh1_4 (Math|Transform|MakeTransform "-52.365536,0.854092,-4.772377" "0,0.000000, 0") false false))
        (:2
          (Components|StaticMesh|SetStaticMesh _staticmesh1_5 "/Game/OldVillage/Meshes/Structure_Components/SM_Bars_002.SM_Bars_002")
          (Transformation|SetRelativeTransform _staticmesh1_5 (Math|Transform|MakeTransform "-58.000000,0.854092,-4.772377" "0,0.000000, 0") false false))
        (:3
          (Components|StaticMesh|SetStaticMesh _staticmesh1_3 "/Game/OldVillage/Meshes/Structure_Components/SM_Bars_001.SM_Bars_001")
          (Transformation|SetRelativeTransform _staticmesh1_3 (Math|Transform|MakeTransform "-52.365536,0.854092,-4.772377" "0,0.000000, 0") false false)))
      (if (Variables|Default|GetAbbandoned%20Building)
        (Rendering|Material|SetMaterial (Variables|Default|GetStaticMesh1) 0 "/Game/OldVillage/Materials/Meshspecific/MI_Fireplace_tools_001_Rusty.MI_Fireplace_tools_001_Rusty"))
      (switch int (Variables|Default|GetChoose%20Window%20Encase)
        (:1
          ;[1 1 1] Encase
          (Components|StaticMesh|SetStaticMesh _staticmesh2_5 "/Game/OldVillage/Meshes/Structure/Decore/SM_Decorative_Stone_010.SM_Decorative_Stone_010")
          (Transformation|SetRelativeTransform _staticmesh2_5 (Math|Transform|MakeTransform "26.695986,-9.927569,50.496395" "90.000000,0.000000, 0" "1.190040,1.240679,1") false false)
          (Components|StaticMesh|SetStaticMesh _staticmesh3_4 "/Game/OldVillage/Meshes/Structure/Decore/SM_Decorative_Stone_007.SM_Decorative_Stone_007")
          (Transformation|SetRelativeTransform _staticmesh3_4 (Math|Transform|MakeTransform "50.516361,-10.543571,77.102379" "0,-89.999992, 0" "0.737631,1.300307,1") false false)
          (Components|StaticMesh|SetStaticMesh _staticmesh4_5 "/Game/OldVillage/Meshes/Structure/Decore/SM_Decorative_Stone_007.SM_Decorative_Stone_007")
          (Transformation|SetRelativeTransform _staticmesh4_5 (Math|Transform|MakeTransform "73.970993,-10.543616,42.740055" "0,-89.999939,89.999962" "-0.737631,1.180277,1") false false)
          (Components|StaticMesh|SetStaticMesh _staticmesh5_4 "/Game/OldVillage/Meshes/Structure/Decore/SM_Decorative_Stone_009.SM_Decorative_Stone_009")
          (Transformation|SetRelativeTransform _staticmesh5_4 (Math|Transform|MakeTransform "44.672520,-9.294608,24.679344" "0,0.000000, 0" "1.439958,1.129181,1") false false))
        (:2
          (Components|StaticMesh|SetStaticMesh _staticmesh2_6 "/Game/OldVillage/Meshes/Structure/Decore/SM_Decorative_Stone_010.SM_Decorative_Stone_010")
          (Transformation|SetRelativeTransform _staticmesh2_6 (Math|Transform|MakeTransform "26.695986,-9.927569,56.147224" "90.000000,0.000000, 0" "1.530136,-1.240679,1") false false)
          (Components|StaticMesh|SetStaticMesh _staticmesh3_5 "/Game/OldVillage/Meshes/Structure/Decore/SM_Decorative_Stone_007.SM_Decorative_Stone_007")
          (Transformation|SetRelativeTransform _staticmesh3_5 (Math|Transform|MakeTransform "55.462299,-10.543571,77.102379" "0,-89.999992, 0" "-0.737631,1.039958,1") false false)
          (Components|StaticMesh|SetStaticMesh _staticmesh4_6 "/Game/OldVillage/Meshes/Structure/Decore/SM_Decorative_Stone_007.SM_Decorative_Stone_007")
          (Transformation|SetRelativeTransform _staticmesh4_6 (Math|Transform|MakeTransform "73.970993,-10.543616,51.934071" "0,-89.999939,89.999962" "-0.737631,0.850274,-1.000000") false false)
          (Components|StaticMesh|SetStaticMesh _staticmesh5_5 "/Game/OldVillage/Meshes/Structure/Decore/SM_Decorative_Stone_009.SM_Decorative_Stone_009")
          (Transformation|SetRelativeTransform _staticmesh5_5 (Math|Transform|MakeTransform "52.302052,-9.294600,24.679344" "0,0.000000, 0" "1.815251,-1.129181,1") false false))
        (:3
          (Components|StaticMesh|SetStaticMesh _staticmesh2 "/Game/OldVillage/Meshes/Structure/Decore/SM_Decorative_Stone_007.SM_Decorative_Stone_007")
          (Transformation|SetRelativeTransform _staticmesh2 (Math|Transform|MakeTransform "26.644115,-10.544028,57.896206" "-0.000034,-89.999939,89.999962" "-0.737631,1.350461,-1.000000") false false)
          (Components|StaticMesh|SetStaticMesh _staticmesh3 "/Game/OldVillage/Meshes/Structure/Decore/SM_Decorative_Stone_009.SM_Decorative_Stone_009")
          (Transformation|SetRelativeTransform _staticmesh3 (Math|Transform|MakeTransform "57.307644,-9.294715,81.930321" "0,0.000000, 0" "1.614788,-1.129181,-1.000000") false false)
          (Components|StaticMesh|SetStaticMesh _staticmesh4 "/Game/OldVillage/Meshes/Structure/Decore/SM_Decorative_Stone_010.SM_Decorative_Stone_010")
          (Transformation|SetRelativeTransform _staticmesh4 (Math|Transform|MakeTransform "77.762634,-9.927615,51.477261" "90.000000,0.000000,0.000000" "1.407300,-1.240679,-1.000000") false false)
          (Components|StaticMesh|SetStaticMesh _staticmesh5 "/Game/OldVillage/Meshes/Structure/Decore/SM_Decorative_Stone_007.SM_Decorative_Stone_007")
          (Transformation|SetRelativeTransform _staticmesh5 (Math|Transform|MakeTransform "52.236000,-10.543471,21.286085" "0,-89.999992, 0" "-0.737631,1.260397,-1.000000") false false))
        (:4
          (if (Variables|Default|GetAbbandoned%20Building)
            (Components|StaticMesh|SetStaticMesh _staticmesh2_4 "/Game/OldVillage/Meshes/Structure_Components/SM_Pole_001_abbandoned.SM_Pole_001_abbandoned")
            (Transformation|SetRelativeTransform _staticmesh2_4 (Math|Transform|MakeTransform "31.146448,2.297110,30.797565" "0.000000,0.000000,0.000000" "0.455762,1.070000,0.499866") false false)
            (Components|StaticMesh|SetStaticMesh _staticmesh3_3 "/Game/OldVillage/Meshes/Structure_Components/SM_Pole_002_abbandoned.SM_Pole_002_abbandoned")
            (Transformation|SetRelativeTransform _staticmesh3_3 (Math|Transform|MakeTransform "31.146444,1.100000,81.246803" "-90.000000,0.000000,-2.000000" "0.545757,1.100000,0.469972") false false)
            (Components|StaticMesh|SetStaticMesh _staticmesh4_4 "/Game/OldVillage/Meshes/Structure_Components/SM_Pole_001_abbandoned.SM_Pole_001_abbandoned")
            (Transformation|SetRelativeTransform _staticmesh4_4 (Math|Transform|MakeTransform "67.683838,3.000000,71.347641" "0.000000,-179.999969,-179.999939" "0.486034,1.100000,0.509895") false false)
            (Components|StaticMesh|SetStaticMesh _staticmesh5_3 "/Game/OldVillage/Meshes/Structure_Components/SM_Pole_002_abbandoned.SM_Pole_002_abbandoned")
            (Transformation|SetRelativeTransform _staticmesh5_3 (Math|Transform|MakeTransform "67.609573,1.000000,20.782869" "90.000000,35.264412,35.264389" "0.545757,1.100000,0.469972") false false)
            (else
              (Components|StaticMesh|SetStaticMesh _staticmesh2_2 "/Game/OldVillage/Meshes/Structure_Components/SM_Pole_001.SM_Pole_001")
              (Transformation|SetRelativeTransform _staticmesh2_2 (Math|Transform|MakeTransform "31.146448,2.297110,30.797565" "0.000000,0.000000,0.000000" "0.455762,1.070000,0.499866") false false)
              (Components|StaticMesh|SetStaticMesh _staticmesh3_2 "/Game/OldVillage/Meshes/Structure_Components/SM_Pole_002.SM_Pole_002")
              (Transformation|SetRelativeTransform _staticmesh3_2 (Math|Transform|MakeTransform "31.146444,1.100000,81.246803" "-90.000000,0.000000,-2.000000" "0.565757,1.100000,0.470000") false false)
              (Components|StaticMesh|SetStaticMesh _staticmesh4_2 "/Game/OldVillage/Meshes/Structure_Components/SM_Pole_001.SM_Pole_001")
              (Transformation|SetRelativeTransform _staticmesh4_2 (Math|Transform|MakeTransform "67.683838,3.000000,71.347641" "0.000000,-179.999969,-179.999939" "0.486034,1.100000,0.509895") false false)
              (Components|StaticMesh|SetStaticMesh _staticmesh5_2 "/Game/OldVillage/Meshes/Structure_Components/SM_Pole_002.SM_Pole_002")
              (Transformation|SetRelativeTransform _staticmesh5_2 (Math|Transform|MakeTransform "67.609573,1.000000,20.782869" "90.000000,35.264412,35.264389" "0.545757,1.100000,0.469972") false false))))))
    (:NewEnumerator1
      ;[1 1 1] Corner R IN
      (if (Variables|Default|GetAbbandoned%20Building)
        (Rendering|Material|SetMaterial (Variables|Default|GetStatic%20Mesh) 0 "/Game/OldVillage/Materials/Tileable/MI_Blend_Stones_Exterior_001_to_Stucco_fine_001_parallax.MI_Blend_Stones_Exterior_001_to_Stucco_fine_001_parallax"))
      (Components|StaticMesh|SetStaticMesh _static_mesh_2 "/Game/OldVillage/Meshes/Structure_Components/SM_Wall_1mx1m_Edge_L_001.SM_Wall_1mx1m_Edge_L_001")
      (Transformation|SetRelativeTransform _static_mesh_2 (Math|Transform|MakeTransform "0.000000,0.000000,0.000000" "0,0.000000, 0" "1,1.000000,1") false false))
    (:NewEnumerator7
      ;[1 1 1] Corner R OUT
      (if (Variables|Default|GetAbbandoned%20Building)
        (Rendering|Material|SetMaterial (Variables|Default|GetStatic%20Mesh) 0 "/Game/OldVillage/Materials/Tileable/MI_Blend_Stones_Exterior_001_to_Stucco_fine_001_parallax.MI_Blend_Stones_Exterior_001_to_Stucco_fine_001_parallax"))
      (Components|StaticMesh|SetStaticMesh _static_mesh_3 "/Game/OldVillage/Meshes/Structure_Components/SM_Wall_1mx1m_Edge_Out_R_001.SM_Wall_1mx1m_Edge_Out_R_001")
      (Transformation|SetRelativeTransform _static_mesh_3 (Math|Transform|MakeTransform "0.000000,0.000000,0.000000" "0,0.000000, 0" "1,1.000000,1") false false))
    (:NewEnumerator2
      ;[1 1 1] Corner L IN
      (if (Variables|Default|GetAbbandoned%20Building)
        (Rendering|Material|SetMaterial (Variables|Default|GetStatic%20Mesh) 0 "/Game/OldVillage/Materials/Tileable/MI_Blend_Stones_Exterior_001_to_Stucco_fine_001_parallax.MI_Blend_Stones_Exterior_001_to_Stucco_fine_001_parallax"))
      (Components|StaticMesh|SetStaticMesh _static_mesh "/Game/OldVillage/Meshes/Structure_Components/SM_Wall_1mx1m_Edge_R_001.SM_Wall_1mx1m_Edge_R_001")
      (Transformation|SetRelativeTransform _static_mesh (Math|Transform|MakeTransform "100.000000,0.000000,0.000000" "0,0.000000, 0" "1,1.000000,1") false false))
    (:NewEnumerator8
      ;[1 1 1] Corner L OUT
      (if (Variables|Default|GetAbbandoned%20Building)
        (Rendering|Material|SetMaterial (Variables|Default|GetStatic%20Mesh) 0 "/Game/OldVillage/Materials/Tileable/MI_Blend_Stones_Exterior_001_to_Stucco_fine_001_parallax.MI_Blend_Stones_Exterior_001_to_Stucco_fine_001_parallax"))
      (Components|StaticMesh|SetStaticMesh _static_mesh_8 "/Game/OldVillage/Meshes/Structure_Components/SM_Wall_1mx1m_Edge_Out_L_001.SM_Wall_1mx1m_Edge_Out_L_001")
      (Transformation|SetRelativeTransform _static_mesh_8 (Math|Transform|MakeTransform "100.000000,0.000000,0.000000" "0,0.000000, 0" "1,1.000000,1") false false))
    (:NewEnumerator11
      ;[1 1 1] Bend
      (if (Variables|Default|GetAbbandoned%20Building)
        (Rendering|Material|SetMaterial (Variables|Default|GetStatic%20Mesh) 1 "/Game/OldVillage/Materials/Tileable/MI_Blend_Stones_Exterior_001_to_Stucco_fine_001_parallax.MI_Blend_Stones_Exterior_001_to_Stucco_fine_001_parallax"))
      (Components|StaticMesh|SetStaticMesh _static_mesh_9 "/Game/OldVillage/Meshes/Structure_Components/SM_Wall_1mx1m_Bend_001.SM_Wall_1mx1m_Bend_001")
      (Transformation|SetRelativeTransform _static_mesh_9 (Math|Transform|MakeTransform "0.000000,0.000000,0.000000" "0,0.000000, 0" "1,1.000000,1") false false))))