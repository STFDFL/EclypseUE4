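; Village fence actor that builds itself along an editable spline in the construction script, with no active runtime logic.
; ChooseFenceStyle selects Flat, Rounded, Sloped or Mixed, and each segment gets a randomly picked spline mesh, unseeded.
; The last point gets a narrow end piece or, with AddGate outside Mixed, two static meshes forming a gate.
; GateRotation1Open0Closed swings one gate mesh by lerping its yaw from closed to open.
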(event EventBeginPlay)

(event EventActorBeginOverlap
  (params (OtherActor :type Actor%20Object%20Reference)))

(event EventTick
  (params (DeltaSeconds :type Float%20%28single-precision%29)))

(fn ConstructionScript
  (bind _spline (Variables|Default|GetSpline))
  (bind _defaultsceneroot (Variables|Default|GetDefaultSceneRoot))
  (bind _spline_2 (Variables|Default|GetSpline))
  (bind _defaultsceneroot_2 (Variables|Default|GetDefaultSceneRoot))
  (bind _spline_3 (Variables|Default|GetSpline))
  (bind _defaultsceneroot_3 (Variables|Default|GetDefaultSceneRoot))
  (bind _defaultsceneroot_4 (Variables|Default|GetDefaultSceneRoot))
  (bind _defaultsceneroot_5 (Variables|Default|GetDefaultSceneRoot))
  (bind _spline_4 (Variables|Default|GetSpline))
  (bind _defaultsceneroot_6 (Variables|Default|GetDefaultSceneRoot))
  (switch Utilities|FlowControl|Switch|SwitchonBP_Fence_Enum (Variables|Default|GetChoose%20Fence%20Style)
    (:NewEnumerator0
      (for _index (range 0 (- (Spline|GetNumberOfSplinePoints (Variables|Default|GetSpline)) 2))
        (switch int (Math|Random|RandomInteger 4)
          (:0
            (bind _returnvalue (AddComponent|AddSplineMeshComponent true))
            (Class|SceneComponent|Attachto _returnvalue _defaultsceneroot_6 "None" "KeepRelativeOffset" true)
            (SplineMesh|SetStartandEnd _returnvalue (.Location (Spline|GetLocationandTangentatSplinePoint _spline_4 _index "Local")) (.Tangent (Spline|GetLocationandTangentatSplinePoint _spline_4 _index "Local")) (- (.Location (Spline|GetLocationandTangentatSplinePoint _spline_4 (+ _index 1) "Local")) "-5.000000,4.000000, 0") (- (.Tangent (Spline|GetLocationandTangentatSplinePoint _spline_4 (+ _index 1) "Local")) "-5.000000,4.000000, 0") true :!class /Script/Engine.SplineMeshComponent))
          (:1
            (bind _returnvalue_2 (AddComponent|AddSplineMeshComponent true))
            (Class|SceneComponent|Attachto _returnvalue_2 _defaultsceneroot_6 "None" "KeepRelativeOffset" true)
            (SplineMesh|SetStartandEnd _returnvalue_2 (.Location (Spline|GetLocationandTangentatSplinePoint _spline_4 _index "Local")) (.Tangent (Spline|GetLocationandTangentatSplinePoint _spline_4 _index "Local")) (- (.Location (Spline|GetLocationandTangentatSplinePoint _spline_4 (+ _index 1) "Local")) "-5.000000,4.000000, 0") (- (.Tangent (Spline|GetLocationandTangentatSplinePoint _spline_4 (+ _index 1) "Local")) "-5.000000,4.000000, 0") true :!class /Script/Engine.SplineMeshComponent))
          (:2
            (bind _returnvalue_3 (AddComponent|AddSplineMeshComponent true))
            (Class|SceneComponent|Attachto _returnvalue_3 _defaultsceneroot_6 "None" "KeepRelativeOffset" true)
            (SplineMesh|SetStartandEnd _returnvalue_3 (.Location (Spline|GetLocationandTangentatSplinePoint _spline_4 _index "Local")) (.Tangent (Spline|GetLocationandTangentatSplinePoint _spline_4 _index "Local")) (- (.Location (Spline|GetLocationandTangentatSplinePoint _spline_4 (+ _index 1) "Local")) "-5.000000,4.000000, 0") (- (.Tangent (Spline|GetLocationandTangentatSplinePoint _spline_4 (+ _index 1) "Local")) "-5.000000,4.000000, 0") true :!class /Script/Engine.SplineMeshComponent))
          (:3
            (bind _returnvalue_4 (AddComponent|AddSplineMeshComponent true))
            (Class|SceneComponent|Attachto _returnvalue_4 _defaultsceneroot_6 "None" "KeepRelativeOffset" true)
            (SplineMesh|SetStartandEnd _returnvalue_4 (.Location (Spline|GetLocationandTangentatSplinePoint _spline_4 _index "Local")) (.Tangent (Spline|GetLocationandTangentatSplinePoint _spline_4 _index "Local")) (- (.Location (Spline|GetLocationandTangentatSplinePoint _spline_4 (+ _index 1) "Local")) "-5.000000,4.000000, 0") (- (.Tangent (Spline|GetLocationandTangentatSplinePoint _spline_4 (+ _index 1) "Local")) "-5.000000,4.000000, 0") true :!class /Script/Engine.SplineMeshComponent))))
      (if (Variables|Default|GetAdd%20Gate)
        (AddComponent|AddStaticMeshComponent false (Math|Transform|MakeTransform (- (- (.Location (Spline|GetLocationandTangentatSplinePoint _spline_4 (+ _index 1) "Local")) "-5.000000,4.000000, 0") "-3.000000,-6.000000, 0") (Spline|GetRotationatSplinePoint (Variables|Default|GetSpline) (+ _index 1) "Local") "1.000000,1.000000,1"))
        (bind _returnvalue_5 (AddComponent|AddStaticMeshComponent false (Math|Transform|MakeTransform (- (- (.Location (Spline|GetLocationandTangentatSplinePoint _spline_4 (+ _index 1) "Local")) "-5.000000,4.000000, 0") "-3.000000,-6.000000, 0") (Spline|GetRotationatSplinePoint (Variables|Default|GetSpline) (+ _index 1) "Local") "1.000000,1.000000,1")))
        (Transformation|AddLocalRotation _returnvalue_5 (Math|Rotator|Lerp(Rotator) (Math|Rotator|MakeRotator 0.0 0.0 0.0) (Math|Rotator|MakeRotator 0.0 0.0 -1.7e+02) (Math|Float|Clamp(Float) (Variables|Default|GetGate%20Rotation%201=%20Open%200=%20Closed))) false false)
        (else
          (AddComponent|AddSplineMeshComponent false (Math|Transform|MakeTransform (- (- (.Location (Spline|GetLocationandTangentatSplinePoint _spline_4 (+ _index 1) "Local")) "-5.000000,4.000000, 0") "0.000000,-6.000000, 0") (Spline|GetRotationatSplinePoint (Variables|Default|GetSpline) (+ _index 1) "Local") "0.150000,1.000000,1")))))
    (:NewEnumerator1
      (for _index_2 (range 0 (- (Spline|GetNumberOfSplinePoints (Variables|Default|GetSpline)) 2))
        (switch int (Math|Random|RandomInteger 4)
          (:0
            (bind _returnvalue_6 (AddComponent|AddSplineMeshComponent true))
            (Class|SceneComponent|Attachto _returnvalue_6 _defaultsceneroot_2 "None" "KeepRelativeOffset" true)
            (SplineMesh|SetStartandEnd _returnvalue_6 (.Location (Spline|GetLocationandTangentatSplinePoint _spline_2 _index_2 "Local")) (.Tangent (Spline|GetLocationandTangentatSplinePoint _spline_2 _index_2 "Local")) (- (.Location (Spline|GetLocationandTangentatSplinePoint _spline_2 (+ _index_2 1) "Local")) "-5.000000,4.000000, 0") (- (.Tangent (Spline|GetLocationandTangentatSplinePoint _spline_2 (+ _index_2 1) "Local")) "-5.000000,4.000000, 0") true :!class /Script/Engine.SplineMeshComponent))
          (:1
            (bind _returnvalue_7 (AddComponent|AddSplineMeshComponent true))
            (Class|SceneComponent|Attachto _returnvalue_7 _defaultsceneroot_2 "None" "KeepRelativeOffset" true)
            (SplineMesh|SetStartandEnd _returnvalue_7 (.Location (Spline|GetLocationandTangentatSplinePoint _spline_2 _index_2 "Local")) (.Tangent (Spline|GetLocationandTangentatSplinePoint _spline_2 _index_2 "Local")) (- (.Location (Spline|GetLocationandTangentatSplinePoint _spline_2 (+ _index_2 1) "Local")) "-5.000000,4.000000, 0") (- (.Tangent (Spline|GetLocationandTangentatSplinePoint _spline_2 (+ _index_2 1) "Local")) "-5.000000,4.000000, 0") true :!class /Script/Engine.SplineMeshComponent))
          (:2
            (bind _returnvalue_8 (AddComponent|AddSplineMeshComponent true))
            (Class|SceneComponent|Attachto _returnvalue_8 _defaultsceneroot_2 "None" "KeepRelativeOffset" true)
            (SplineMesh|SetStartandEnd _returnvalue_8 (.Location (Spline|GetLocationandTangentatSplinePoint _spline_2 _index_2 "Local")) (.Tangent (Spline|GetLocationandTangentatSplinePoint _spline_2 _index_2 "Local")) (- (.Location (Spline|GetLocationandTangentatSplinePoint _spline_2 (+ _index_2 1) "Local")) "-5.000000,4.000000, 0") (- (.Tangent (Spline|GetLocationandTangentatSplinePoint _spline_2 (+ _index_2 1) "Local")) "-5.000000,4.000000, 0") true :!class /Script/Engine.SplineMeshComponent))
          (:3
            (bind _returnvalue_9 (AddComponent|AddSplineMeshComponent true))
            (Class|SceneComponent|Attachto _returnvalue_9 _defaultsceneroot_2 "None" "KeepRelativeOffset" true)
            (SplineMesh|SetStartandEnd _returnvalue_9 (.Location (Spline|GetLocationandTangentatSplinePoint _spline_2 _index_2 "Local")) (.Tangent (Spline|GetLocationandTangentatSplinePoint _spline_2 _index_2 "Local")) (- (.Location (Spline|GetLocationandTangentatSplinePoint _spline_2 (+ _index_2 1) "Local")) "-5.000000,4.000000, 0") (- (.Tangent (Spline|GetLocationandTangentatSplinePoint _spline_2 (+ _index_2 1) "Local")) "-5.000000,4.000000, 0") true :!class /Script/Engine.SplineMeshComponent))))
      (if (Variables|Default|GetAdd%20Gate)
        (AddComponent|AddStaticMeshComponent false (Math|Transform|MakeTransform (- (- (.Location (Spline|GetLocationandTangentatSplinePoint _spline_2 (+ _index_2 1) "Local")) "-5.000000,4.000000, 0") "-6.000000,-7.000000, 0") (Spline|GetRotationatSplinePoint (Variables|Default|GetSpline) (+ _index_2 1) "Local") "1.000000,1.000000,1"))
        (bind _returnvalue_10 (AddComponent|AddStaticMeshComponent false (Math|Transform|MakeTransform (- (- (.Location (Spline|GetLocationandTangentatSplinePoint _spline_2 (+ _index_2 1) "Local")) "-5.000000,4.000000, 0") "-6.000000,-7.000000, 0") (Spline|GetRotationatSplinePoint (Variables|Default|GetSpline) (+ _index_2 1) "Local") "1.000000,1.000000,1")))
        (Transformation|AddLocalRotation _returnvalue_10 (Math|Rotator|Lerp(Rotator) (Math|Rotator|MakeRotator 0.0 0.0 0.0) (Math|Rotator|MakeRotator 0.0 0.0 -1.7e+02) (Math|Float|Clamp(Float) (Variables|Default|GetGate%20Rotation%201=%20Open%200=%20Closed))) false false)
        (else
          (AddComponent|AddSplineMeshComponent false (Math|Transform|MakeTransform (- (- (.Location (Spline|GetLocationandTangentatSplinePoint _spline_2 (+ _index_2 1) "Local")) "-5.000000,4.000000, 0") "0.000000,-6.000000, 0") (Spline|GetRotationatSplinePoint (Variables|Default|GetSpline) (+ _index_2 1) "Local") "0.150000,1.000000,1")))))
    (:NewEnumerator2
      (for _index_3 (range 0 (- (Spline|GetNumberOfSplinePoints (Variables|Default|GetSpline)) 2))
        (switch int (Math|Random|RandomInteger 4)
          (:0
            (bind _returnvalue_11 (AddComponent|AddSplineMeshComponent true))
            (Class|SceneComponent|Attachto _returnvalue_11 _defaultsceneroot_3 "None" "KeepRelativeOffset" true)
            (SplineMesh|SetStartandEnd _returnvalue_11 (.Location (Spline|GetLocationandTangentatSplinePoint _spline_3 _index_3 "Local")) (.Tangent (Spline|GetLocationandTangentatSplinePoint _spline_3 _index_3 "Local")) (- (.Location (Spline|GetLocationandTangentatSplinePoint _spline_3 (+ _index_3 1) "Local")) "-5.000000,4.000000, 0") (- (.Tangent (Spline|GetLocationandTangentatSplinePoint _spline_3 (+ _index_3 1) "Local")) "-5.000000,4.000000, 0") true :!class /Script/Engine.SplineMeshComponent))
          (:1
            (bind _returnvalue_12 (AddComponent|AddSplineMeshComponent true))
            (Class|SceneComponent|Attachto _returnvalue_12 _defaultsceneroot_3 "None" "KeepRelativeOffset" true)
            (SplineMesh|SetStartandEnd _returnvalue_12 (.Location (Spline|GetLocationandTangentatSplinePoint _spline_3 _index_3 "Local")) (.Tangent (Spline|GetLocationandTangentatSplinePoint _spline_3 _index_3 "Local")) (- (.Location (Spline|GetLocationandTangentatSplinePoint _spline_3 (+ _index_3 1) "Local")) "-5.000000,4.000000, 0") (- (.Tangent (Spline|GetLocationandTangentatSplinePoint _spline_3 (+ _index_3 1) "Local")) "-5.000000,4.000000, 0") true :!class /Script/Engine.SplineMeshComponent))
          (:2
            (bind _returnvalue_13 (AddComponent|AddSplineMeshComponent true))
            (Class|SceneComponent|Attachto _returnvalue_13 _defaultsceneroot_3 "None" "KeepRelativeOffset" true)
            (SplineMesh|SetStartandEnd _returnvalue_13 (.Location (Spline|GetLocationandTangentatSplinePoint _spline_3 _index_3 "Local")) (.Tangent (Spline|GetLocationandTangentatSplinePoint _spline_3 _index_3 "Local")) (- (.Location (Spline|GetLocationandTangentatSplinePoint _spline_3 (+ _index_3 1) "Local")) "-5.000000,4.000000, 0") (- (.Tangent (Spline|GetLocationandTangentatSplinePoint _spline_3 (+ _index_3 1) "Local")) "-5.000000,4.000000, 0") true :!class /Script/Engine.SplineMeshComponent))
          (:3
            (bind _returnvalue_14 (AddComponent|AddSplineMeshComponent true))
            (Class|SceneComponent|Attachto _returnvalue_14 _defaultsceneroot_3 "None" "KeepRelativeOffset" true)
            (SplineMesh|SetStartandEnd _returnvalue_14 (.Location (Spline|GetLocationandTangentatSplinePoint _spline_3 _index_3 "Local")) (.Tangent (Spline|GetLocationandTangentatSplinePoint _spline_3 _index_3 "Local")) (- (.Location (Spline|GetLocationandTangentatSplinePoint _spline_3 (+ _index_3 1) "Local")) "-5.000000,4.000000, 0") (- (.Tangent (Spline|GetLocationandTangentatSplinePoint _spline_3 (+ _index_3 1) "Local")) "-5.000000,4.000000, 0") true :!class /Script/Engine.SplineMeshComponent))))
      (if (Variables|Default|GetAdd%20Gate)
        (AddComponent|AddStaticMeshComponent false (Math|Transform|MakeTransform (- (- (- (.Location (Spline|GetLocationandTangentatSplinePoint _spline_3 (+ _index_3 1) "Local")) "-5.000000,4.000000, 0") "0.000000,-6.000000, 0") "-7.000000,2.000000,0.000000") (Spline|GetRotationatSplinePoint (Variables|Default|GetSpline) (+ _index_3 1) "Local") "1.000000,1.000000,1"))
        (bind _returnvalue_15 (AddComponent|AddStaticMeshComponent false (Math|Transform|MakeTransform (- (- (- (.Location (Spline|GetLocationandTangentatSplinePoint _spline_3 (+ _index_3 1) "Local")) "-5.000000,4.000000, 0") "0.000000,-6.000000, 0") "-7.000000,2.000000,0.000000") (Spline|GetRotationatSplinePoint (Variables|Default|GetSpline) (+ _index_3 1) "Local") "1.000000,1.000000,1")))
        (Transformation|AddLocalRotation _returnvalue_15 (Math|Rotator|Lerp(Rotator) (Math|Rotator|MakeRotator 0.0 0.0 0.0) (Math|Rotator|MakeRotator 0.0 0.0 -1.7e+02) (Math|Float|Clamp(Float) (Variables|Default|GetGate%20Rotation%201=%20Open%200=%20Closed))) false false)
        (else
          (AddComponent|AddSplineMeshComponent false (Math|Transform|MakeTransform (- (- (.Location (Spline|GetLocationandTangentatSplinePoint _spline_3 (+ _index_3 1) "Local")) "-5.000000,4.000000, 0") "0.000000,-6.000000, 0") (Spline|GetRotationatSplinePoint (Variables|Default|GetSpline) (+ _index_3 1) "Local") "0.150000,1.000000,1")))))
    (:NewEnumerator3
      (for _index_4 (range 0 (- (Spline|GetNumberOfSplinePoints (Variables|Default|GetSpline)) 2))
        (switch int (Math|Random|RandomInteger 12)
          (:0
            (bind _returnvalue_16 (AddComponent|AddSplineMeshComponent true))
            (Class|SceneComponent|Attachto _returnvalue_16 _defaultsceneroot_4 "None" "KeepRelativeOffset" true)
            (SplineMesh|SetStartandEnd _returnvalue_16 (.Location (Spline|GetLocationandTangentatSplinePoint _spline _index_4 "Local")) (.Tangent (Spline|GetLocationandTangentatSplinePoint _spline _index_4 "Local")) (- (.Location (Spline|GetLocationandTangentatSplinePoint _spline (+ _index_4 1) "Local")) "-5.000000,4.000000, 0") (- (.Tangent (Spline|GetLocationandTangentatSplinePoint _spline (+ _index_4 1) "Local")) "-5.000000,4.000000, 0") true :!class /Script/Engine.SplineMeshComponent))
          (:1
            (bind _returnvalue_17 (AddComponent|AddSplineMeshComponent true))
            (Class|SceneComponent|Attachto _returnvalue_17 _defaultsceneroot_4 "None" "KeepRelativeOffset" true)
            (SplineMesh|SetStartandEnd _returnvalue_17 (.Location (Spline|GetLocationandTangentatSplinePoint _spline _index_4 "Local")) (.Tangent (Spline|GetLocationandTangentatSplinePoint _spline _index_4 "Local")) (- (.Location (Spline|GetLocationandTangentatSplinePoint _spline (+ _index_4 1) "Local")) "-5.000000,4.000000, 0") (- (.Tangent (Spline|GetLocationandTangentatSplinePoint _spline (+ _index_4 1) "Local")) "-5.000000,4.000000, 0") true :!class /Script/Engine.SplineMeshComponent))
          (:2
            (bind _returnvalue_18 (AddComponent|AddSplineMeshComponent true))
            (Class|SceneComponent|Attachto _returnvalue_18 _defaultsceneroot_4 "None" "KeepRelativeOffset" true)
            (SplineMesh|SetStartandEnd _returnvalue_18 (.Location (Spline|GetLocationandTangentatSplinePoint _spline _index_4 "Local")) (.Tangent (Spline|GetLocationandTangentatSplinePoint _spline _index_4 "Local")) (- (.Location (Spline|GetLocationandTangentatSplinePoint _spline (+ _index_4 1) "Local")) "-5.000000,4.000000, 0") (- (.Tangent (Spline|GetLocationandTangentatSplinePoint _spline (+ _index_4 1) "Local")) "-5.000000,4.000000, 0") true :!class /Script/Engine.SplineMeshComponent))
          (:3
            (bind _returnvalue_19 (AddComponent|AddSplineMeshComponent true))
            (Class|SceneComponent|Attachto _returnvalue_19 _defaultsceneroot_4 "None" "KeepRelativeOffset" true)
            (SplineMesh|SetStartandEnd _returnvalue_19 (.Location (Spline|GetLocationandTangentatSplinePoint _spline _index_4 "Local")) (.Tangent (Spline|GetLocationandTangentatSplinePoint _spline _index_4 "Local")) (- (.Location (Spline|GetLocationandTangentatSplinePoint _spline (+ _index_4 1) "Local")) "-5.000000,4.000000, 0") (- (.Tangent (Spline|GetLocationandTangentatSplinePoint _spline (+ _index_4 1) "Local")) "-5.000000,4.000000, 0") true :!class /Script/Engine.SplineMeshComponent))
          (:4
            (bind _returnvalue_20 (AddComponent|AddSplineMeshComponent true))
            (Class|SceneComponent|Attachto _returnvalue_20 _defaultsceneroot_5 "None" "KeepRelativeOffset" true)
            (SplineMesh|SetStartandEnd _returnvalue_20 (.Location (Spline|GetLocationandTangentatSplinePoint _spline _index_4 "Local")) (.Tangent (Spline|GetLocationandTangentatSplinePoint _spline _index_4 "Local")) (- (.Location (Spline|GetLocationandTangentatSplinePoint _spline (+ _index_4 1) "Local")) "-5.000000,4.000000, 0") (- (.Tangent (Spline|GetLocationandTangentatSplinePoint _spline (+ _index_4 1) "Local")) "-5.000000,4.000000, 0") true :!class /Script/Engine.SplineMeshComponent))
          (:5
            (bind _returnvalue_21 (AddComponent|AddSplineMeshComponent true))
            (Class|SceneComponent|Attachto _returnvalue_21 _defaultsceneroot_5 "None" "KeepRelativeOffset" true)
            (SplineMesh|SetStartandEnd _returnvalue_21 (.Location (Spline|GetLocationandTangentatSplinePoint _spline _index_4 "Local")) (.Tangent (Spline|GetLocationandTangentatSplinePoint _spline _index_4 "Local")) (- (.Location (Spline|GetLocationandTangentatSplinePoint _spline (+ _index_4 1) "Local")) "-5.000000,4.000000, 0") (- (.Tangent (Spline|GetLocationandTangentatSplinePoint _spline (+ _index_4 1) "Local")) "-5.000000,4.000000, 0") true :!class /Script/Engine.SplineMeshComponent))
          (:6
            (bind _returnvalue_22 (AddComponent|AddSplineMeshComponent true))
            (Class|SceneComponent|Attachto _returnvalue_22 _defaultsceneroot_5 "None" "KeepRelativeOffset" true)
            (SplineMesh|SetStartandEnd _returnvalue_22 (.Location (Spline|GetLocationandTangentatSplinePoint _spline _index_4 "Local")) (.Tangent (Spline|GetLocationandTangentatSplinePoint _spline _index_4 "Local")) (- (.Location (Spline|GetLocationandTangentatSplinePoint _spline (+ _index_4 1) "Local")) "-5.000000,4.000000, 0") (- (.Tangent (Spline|GetLocationandTangentatSplinePoint _spline (+ _index_4 1) "Local")) "-5.000000,4.000000, 0") true :!class /Script/Engine.SplineMeshComponent))
          (:7
            (bind _returnvalue_23 (AddComponent|AddSplineMeshComponent true))
            (Class|SceneComponent|Attachto _returnvalue_23 _defaultsceneroot_5 "None" "KeepRelativeOffset" true)
            (SplineMesh|SetStartandEnd _returnvalue_23 (.Location (Spline|GetLocationandTangentatSplinePoint _spline _index_4 "Local")) (.Tangent (Spline|GetLocationandTangentatSplinePoint _spline _index_4 "Local")) (- (.Location (Spline|GetLocationandTangentatSplinePoint _spline (+ _index_4 1) "Local")) "-5.000000,4.000000, 0") (- (.Tangent (Spline|GetLocationandTangentatSplinePoint _spline (+ _index_4 1) "Local")) "-5.000000,4.000000, 0") true :!class /Script/Engine.SplineMeshComponent))
          (:8
            (bind _returnvalue_24 (AddComponent|AddSplineMeshComponent true))
            (Class|SceneComponent|Attachto _returnvalue_24 _defaultsceneroot "None" "KeepRelativeOffset" true)
            (SplineMesh|SetStartandEnd _returnvalue_24 (.Location (Spline|GetLocationandTangentatSplinePoint _spline _index_4 "Local")) (.Tangent (Spline|GetLocationandTangentatSplinePoint _spline _index_4 "Local")) (- (.Location (Spline|GetLocationandTangentatSplinePoint _spline (+ _index_4 1) "Local")) "-5.000000,4.000000, 0") (- (.Tangent (Spline|GetLocationandTangentatSplinePoint _spline (+ _index_4 1) "Local")) "-5.000000,4.000000, 0") true :!class /Script/Engine.SplineMeshComponent))
          (:9
            (bind _returnvalue_25 (AddComponent|AddSplineMeshComponent true))
            (Class|SceneComponent|Attachto _returnvalue_25 _defaultsceneroot "None" "KeepRelativeOffset" true)
            (SplineMesh|SetStartandEnd _returnvalue_25 (.Location (Spline|GetLocationandTangentatSplinePoint _spline _index_4 "Local")) (.Tangent (Spline|GetLocationandTangentatSplinePoint _spline _index_4 "Local")) (- (.Location (Spline|GetLocationandTangentatSplinePoint _spline (+ _index_4 1) "Local")) "-5.000000,4.000000, 0") (- (.Tangent (Spline|GetLocationandTangentatSplinePoint _spline (+ _index_4 1) "Local")) "-5.000000,4.000000, 0") true :!class /Script/Engine.SplineMeshComponent))
          (:10
            (bind _returnvalue_26 (AddComponent|AddSplineMeshComponent true))
            (Class|SceneComponent|Attachto _returnvalue_26 _defaultsceneroot "None" "KeepRelativeOffset" true)
            (SplineMesh|SetStartandEnd _returnvalue_26 (.Location (Spline|GetLocationandTangentatSplinePoint _spline _index_4 "Local")) (.Tangent (Spline|GetLocationandTangentatSplinePoint _spline _index_4 "Local")) (- (.Location (Spline|GetLocationandTangentatSplinePoint _spline (+ _index_4 1) "Local")) "-5.000000,4.000000, 0") (- (.Tangent (Spline|GetLocationandTangentatSplinePoint _spline (+ _index_4 1) "Local")) "-5.000000,4.000000, 0") true :!class /Script/Engine.SplineMeshComponent))
          (:11
            (bind _returnvalue_27 (AddComponent|AddSplineMeshComponent true))
            (Class|SceneComponent|Attachto _returnvalue_27 _defaultsceneroot "None" "KeepRelativeOffset" true)
            (SplineMesh|SetStartandEnd _returnvalue_27 (.Location (Spline|GetLocationandTangentatSplinePoint _spline _index_4 "Local")) (.Tangent (Spline|GetLocationandTangentatSplinePoint _spline _index_4 "Local")) (- (.Location (Spline|GetLocationandTangentatSplinePoint _spline (+ _index_4 1) "Local")) "-5.000000,4.000000, 0") (- (.Tangent (Spline|GetLocationandTangentatSplinePoint _spline (+ _index_4 1) "Local")) "-5.000000,4.000000, 0") true :!class /Script/Engine.SplineMeshComponent))))
      (switch int (Math|Random|RandomInteger 2)
        (:0
          (AddComponent|AddSplineMeshComponent false (Math|Transform|MakeTransform (- (- (.Location (Spline|GetLocationandTangentatSplinePoint _spline (+ _index_4 1) "Local")) "-5.000000,4.000000, 0") "0.000000,-6.000000, 0") (Spline|GetRotationatSplinePoint (Variables|Default|GetSpline) (+ _index_4 1) "Local") "0.150000,1.000000,1")))
        (:1
          (AddComponent|AddSplineMeshComponent false (Math|Transform|MakeTransform (- (- (.Location (Spline|GetLocationandTangentatSplinePoint _spline (+ _index_4 1) "Local")) "-5.000000,4.000000, 0") "0.000000,-6.000000, 0") (Spline|GetRotationatSplinePoint (Variables|Default|GetSpline) (+ _index_4 1) "Local") "0.150000,1.000000,1")))))))