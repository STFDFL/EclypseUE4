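; BP_Well is a village well structure that shows a name label on cursor hover.
; Hovering its cylinder sets the town widget's name slot to "Pyre", reveals a 3D label and turns the text toward the player camera once.
; Leaving clears the name and hides the label and the widget's PyreButton.
; The construction script toggles ivy visibility and offsets the water by WaterHeight along local Y.
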(event OnBeginCursorOver(Cilinder)
  (params (TouchedComponent :type Primitive%20Component%20Object%20Reference))
  (bind _textrender (Variables|Default|GetTextRender))
  (bind _asgame_manager (Utilities|Casting|CastToGameManager (Game|GetGameMode)))
  (Rendering|Components|TextRender|SetText (Variables|/Game/BP/Widgets/MainWidget.MainWidget_C|GetBuildingNameSlot (Variables|/Game/BP/GameManager.GameManager_C|GetTownWidget _asgame_manager)) "Pyre")
  (bind _ascamera_actor_bp (Utilities|Casting|CastToCameraActor_BP (Game|Player|GetPlayerPawn 0)))
  (Rendering|SetVisibility _textrender true false)
  (Rendering|SetVisibility (Variables|Default|GetTextBackgrund) true false)
  (Transformation|SetWorldRotation _textrender (Math|Rotator|FindLookatRotation (Transformation|GetWorldLocation _textrender) (Transformation|GetWorldLocation (Variables|/Game/BP/CameraActor_BP.CameraActor_BP_C|GetCamera _ascamera_actor_bp))) false false))

(event OnEndCursorOver(Cilinder)
  (params (TouchedComponent :type Primitive%20Component%20Object%20Reference))
  (bind _asgame_manager (Utilities|Casting|CastToGameManager (Game|GetGameMode)))
  (Rendering|Components|TextRender|SetText (Variables|/Game/BP/Widgets/MainWidget.MainWidget_C|GetBuildingNameSlot (Variables|/Game/BP/GameManager.GameManager_C|GetTownWidget _asgame_manager)) "")
  (Widget|SetVisibility (Variables|/Game/BP/Widgets/MainWidget.MainWidget_C|GetPyreButton (Variables|/Game/BP/GameManager.GameManager_C|GetTownWidget _asgame_manager)) "Hidden")
  (Rendering|SetVisibility (Variables|Default|GetTextRender) false false)
  (Rendering|SetVisibility (Variables|Default|GetTextBackgrund) false false))

(event EventBeginPlay)

(event EventActorBeginOverlap
  (params (OtherActor :type Actor%20Object%20Reference)))

(event EventTick
  (params (DeltaSeconds :type Float%20%28single-precision%29)))

(fn ConstructionScript
  (if (Variables|Default|GetIvy%20)
    (Rendering|SetVisibility (Variables|Default|GetIvy) true false)
    (else
      (Rendering|SetVisibility (Variables|Default|GetIvy) false false)))
  (Transformation|AddLocalOffset (Variables|Default|GetWater) (Math|Vector|MakeVector 0.0 (Math|Conversions|ToFloat(Integer) (Variables|Default|GetWater%20Height)) 0.0) false false))